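; BP_Ball is a bouncing ball that moves in a straight line and disappears after a limited number of overlaps.
; Each Tick it sweeps Sphere1 along Direction at Speed, scaled by delta time, and reflects Direction off the surface normal on a blocking hit.
; Each actor overlap decrements NumberBefourDistr; once it is below one, the next overlap hides Sphere1 without destroying the actor or stopping its movement.
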(event `self.ReceiveActorBeginOverlap`
  (params (OtherActor :type "Actor Object Reference"))
  (if (>= (`self.Number befour distr`) 1)
    (set `self.Number befour distr` (- (`self.Number befour distr`) 1))
    (else
      (`SceneComponent.SetVisibility` (`self.Sphere1`) false false))))

(event `self.ReceiveTick`
  (params (DeltaSeconds :type "Float (single-precision)"))
  (bind _sweephitresult (`SceneComponent.K2_AddWorldOffset` (`self.Sphere1`) (* (* (`self.Direction`) (`self.Speed`)) DeltaSeconds) true false))
  (bind (_bblockinghit _binitialoverlap _time _distance _location _impactpoint _normal) (`GameplayStatics.BreakHitResult` _sweephitresult))
  (if _bblockinghit
    (set `self.Direction` (`KismetMathLibrary.GetReflectionVector` (`self.Direction`) _normal))))

(fn `UserConstructionScript`)